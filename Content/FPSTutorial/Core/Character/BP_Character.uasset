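; First-person player character handling Enhanced Input movement, health, crouch, sprint and interaction.
; SpawnInventory attaches weapons to the arms; messages drive firing, reloading and switching alongside montages, with Tick traces blocking fire near walls and detecting ammo boxes.
; Wall running uses hit normals, plane constraints and reduced gravity.
; Timelines drive aim FOV, power-draining time dilation and active camo, which flip-flops as the crouch timeline finishes and drops on firing.
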(event `EnhancedInput|/Game/FPSTutorial/Data/IA_hurt`
  (params (ActionValue :type Boolean) (ElapsedSeconds :type "Float (double-precision)") (TriggeredSeconds :type "Float (double-precision)") (InputAction :type "InputAction Object Reference" :default "/Game/FPSTutorial/Data/IA_hurt.IA_hurt"))
  (:`Triggered`
    (`/Engine/EditorBlueprintResources/StandardMacros.DoOnce` false :!label _label
      (:`Completed`
        (bind _returnvalue (`GameplayStatics.GetActorOfClass` "/Game/FPSTutorial/Core/Enemy/BP_Enemy_Base.BP_Enemy_Base_C"))
        (bind _asaic_enemy_base (cast `/Game/FPSTutorial/Core/Enemy/AI/AIC_Enemy_Base` (`AIBlueprintHelperLibrary.GetAIController` _returnvalue)))
        (`/Engine/EditorBlueprintResources/StandardMacros.FlipFlop`
          (:`A`
            (`/Game/FPSTutorial/Core/Enemy/AI/AIC_Enemy_Base.SetStateAsAttacking` _asaic_enemy_base self))
          (:`B`
            (`/Game/FPSTutorial/Core/Enemy/AI/AIC_Enemy_Base.SetStateAsPassive` _asaic_enemy_base))))))
  (:`Completed`
    (goto _label :!via `Reset`)))

(event `self.ReceiveAnyDamage`
  (params (Damage :type "Float (single-precision)") (DamageType :type "DamageType Object Reference") (InstigatedBy :type "Controller Object Reference") (DamageCauser :type "Actor Object Reference"))
  (bind _currenthealth (`self.CurrentHealth`))
  (bind _invulnerable (`self.invulnerable`))
  (if (not _invulnerable)
    (set `self.CurrentHealth` (- _currenthealth Damage))
    (if (and (<= _currenthealth 0.0) (not _invulnerable))
      (set `self.CurrentHealth` 0.0)
      (`KismetSystemLibrary.PrintString` "You Died"))))

(event `self.ReceiveBeginPlay`
  (bind _returnvalue (`GameplayStatics.GetPlayerCameraManager` 0))
  (set `PlayerCameraManager.ViewPitchMax` 80.0 _returnvalue)
  (set `PlayerCameraManager.ViewPitchMin` -85.0 _returnvalue)
  (`EnhancedInputSubsystemInterface.AddMappingContext` (pcsubsystem `EnhancedInputLocalPlayerSubsystem` (`GameplayStatics.GetPlayerController` 0)) "/Game/FPSTutorial/Data/IMC_FPS.IMC_FPS" 0 (struct))
  (`self.SpawnInventory`)
  (`self.HolsterToggle`)
  (set `self.CurrentHealth` (`KismetMathLibrary.Conv_IntToDouble` (`self.MaxHealth`)))
  (set `self.CurrentArmour` (`KismetMathLibrary.Conv_IntToDouble` (`self.MaxArmour`)))
  (set `self.currentPower` (`KismetMathLibrary.Conv_IntToDouble` (`self.maxPower`)))
  (`self.InitCamoMats`))

(event `EnhancedInput|/Game/FPSTutorial/Data/IA_ControlTime`
  (params (ActionValue :type Boolean) (ElapsedSeconds :type "Float (double-precision)") (TriggeredSeconds :type "Float (double-precision)") (InputAction :type "InputAction Object Reference" :default "/Game/FPSTutorial/Data/IA_ControlTime.IA_ControlTime"))
  (bind _timecontrolon (`self.TimeControlOn`))
  (:`Triggered`
    (`/Engine/EditorBlueprintResources/StandardMacros.DoOnce` false :!label _label_2
      (:`Completed`
        (`/Engine/EditorBlueprintResources/StandardMacros.FlipFlop`
          (:`A`
            (if (> (`self.currentPower`) 0.0)
              (set `self.TimeControlOn` true)
              (bind (_direction _globaldilation) (`Timeline|TimeControlSpeed` :!label _label_3)
                (:`Update`
                  (`GameplayStatics.SetGlobalTimeDilation` _globaldilation)
                  (set `Actor.CustomTimeDilation` (`KismetMathLibrary.SelectFloat` 3.0 1.0 _timecontrolon) (`GameplayStatics.GetPlayerController` 0))
                  (if _timecontrolon
                    (`|ExecutionSequence`
                      (:`then_0`
                        (if (`self.TimeControlOn`) :!label _label_4
                          (set `self.currentPower` (- (`self.currentPower`) (`self.TimeControlPowerCost`)))
                          (`KismetSystemLibrary.Delay` 0.1)
                          (if (> (`self.currentPower`) 0.0)
                            (goto _label_4)
                            (else
                              (set `self.TimeControlOn` false :!label _label_5)
                              (goto _label_3 :!via `Reverse`)))))
                      (:`then_1`
                        (if (not (`self.bAiming`))
                          (bind (_direction_2 _track0) (`Timeline|TimeControlFOV` :!label _label_6)
                            (:`Update`
                              (`CameraComponent.SetFieldOfView` (`self.Camera`) _track0)))))
                      (:`then_2`
                        (bind (_direction_3 _chromatic_aberration _bloom _vignette) (`Timeline|TimeControlPostProcess` :!label _label_7)
                          (:`Update`
                            (set `CameraComponent.PostProcessSettings` (make `PostProcessSettings` :`SceneFringeIntensity` _chromatic_aberration :`BloomIntensity` _bloom :`VignetteIntensity` _vignette) (`self.Camera`))))))
                    (else
                      (`|ExecutionSequence`
                        (:`then_0`
                          (if (not (`self.bAiming`))
                            (goto _label_6 :!via `Reverse`)))
                        (:`then_1`
                          (goto _label_7 :!via `Reverse`)))))))))
          (:`B`
            (goto _label_5))))))
  (:`Completed`
    (goto _label_2 :!via `Reset`)))

(event `EnhancedInput|/Game/FPSTutorial/Data/IA_Shoot`
  (params (ActionValue :type Boolean) (ElapsedSeconds :type "Float (double-precision)") (TriggeredSeconds :type "Float (double-precision)") (InputAction :type "InputAction Object Reference" :default "/Game/FPSTutorial/Data/IA_Shoot.IA_Shoot"))
  (:`Triggered`
    (`/Engine/EditorBlueprintResources/StandardMacros.DoOnce` false :!label _label_8
      (:`Completed`
        (set `self.bHoldShoot` true)
        (if (and (`self.bHoldShoot`) (not (`self.bCloseToWall`)) (not (`self.bSprinting`)) (> (`self.CurrentAmmo`) 0) (not (`self.bReloading`)) (`self.bEquipped`)) :!label _label_9
          (message `/Game/FPSTutorial/Core/BPI_Weapon.Shoot` (`|GetArrayItem` (`self.EquippedWeapons`) (`self.EquipIndex`)))
          (`|PlayMontage` (`self.CharacterArms`) (select `int` (`self.EquipIndex`) :`0` "/Game/FPSTutorial/Art/Gun/Animations/AM_FP_Gun_Fire.AM_FP_Gun_Fire" :`1` "/Game/FPSTutorial/Art/Glock18/Animations/AM_FP_Glock_Fire.AM_FP_Glock_Fire" :!type "AnimMontage Object Reference")
            (:`then`
              (bind _returnvalue (`GameplayStatics.SpawnEmitterAttached` "/Game/StarterContent/Particles/P_Explosion.P_Explosion" (`Actor.RootComponent` (`|GetArrayItem` (`self.EquippedWeapons`) (`self.EquipIndex`))) "None" (0.0 80.0 0.0) (struct) (0.08 0.08 0.08) "SnapToTargetIncludingScale"))
              (set `ParticleSystemComponent.CustomTimeDilation` 3.0 _returnvalue)
              (`self.DisableCamo`)
              (`KismetSystemLibrary.Delay` (`self.FireDelay`))
              (goto _label_9)))))))
  (:`Completed`
    (set `self.bHoldShoot` false)
    (goto _label_8 :!via `Reset`)))

(event `self.ReceiveTick`
  (params (DeltaSeconds :type "Float (single-precision)"))
  (bind _camera (`self.Camera`))
  (bind _interactdistance (`self.InteractDistance`))
  (bind _returnvalue (`SceneComponent.K2_GetComponentLocation` (`self.Camera`)))
  (bind _returnvalue_2 (`SceneComponent.K2_GetComponentLocation` _camera))
  (bind _returnvalue_3 (`SceneComponent.GetForwardVector` _camera))
  (`SceneComponent.K2_SetRelativeRotation` (`self.Pivot`) (`KismetMathLibrary.MakeRotator` 0.0 (.pitch (`self.GetControlRotation`))) false false)
  (bind (_outhit _returnvalue_4) (`KismetSystemLibrary.LineTraceSingle` _returnvalue (+ _returnvalue_2 (* _returnvalue_3 (80.0 80.0 80.0))) "TraceTypeQuery1"))
  (set `self.bCloseToWall` _returnvalue_4)
  (bind (_outhit_2 _returnvalue_5) (`KismetSystemLibrary.LineTraceSingle` _returnvalue (+ _returnvalue_2 (* _returnvalue_3 (`KismetMathLibrary.MakeVector` _interactdistance _interactdistance _interactdistance))) "TraceTypeQuery1"))
  (bind _output_get (set `self.Interactable` _outhit_2))
  (bind _asbp_ammo_box_interactable (cast `/Game/FPSTutorial/Core/BP_AmmoBox_Interactable` (`.HitActor` (`GameplayStatics.BreakHitResult` _output_get)))
    (:`then`
      (set `self.FoundInteractable` (and _returnvalue_5 (!= (`/Game/FPSTutorial/Core/BP_AmmoBox_Interactable.MaxAmmoOfType` _asbp_ammo_box_interactable) 0))))
    (:`CastFailed`
      (set `self.FoundInteractable` false)))
  (set `self.bEmpty` (== (`self.CurrentAmmo`) 0)))

(event `self.ReceiveHit`
  (params (MyComp :type "PrimitiveComponent Object Reference") (Other :type "Actor Object Reference") (OtherComp :type "PrimitiveComponent Object Reference") (bSelfMoved :type Boolean) (HitLocation :type "Vector Structure") (HitNormal :type "Vector Structure") (NormalImpulse :type "Vector Structure") (Hit :type "HitResult Structure (by ref)"))
  (if (`.IsWall` (`self.CheckForWall` Hit))
    (`self.StartWallRun` HitNormal)
    (else
      (`self.StopWallRun`))))

(event `EnhancedInput|/Game/FPSTutorial/Data/IA_Aim`
  (params (ActionValue :type Boolean) (ElapsedSeconds :type "Float (double-precision)") (TriggeredSeconds :type "Float (double-precision)") (InputAction :type "InputAction Object Reference" :default "/Game/FPSTutorial/Data/IA_Aim.IA_Aim"))
  (:`Triggered`
    (`/Engine/EditorBlueprintResources/StandardMacros.DoOnce` false :!label _label_10
      (:`Completed`
        (`/Engine/EditorBlueprintResources/StandardMacros.FlipFlop`
          (:`A`
            (set `self.bAiming` true)
            (bind (_direction _fov) (`Timeline|AimTimeline` :!via `Reverse` :!label _label_11)
              (:`Update`
                (`CameraComponent.SetFieldOfView` (`self.Camera`) _fov))))
          (:`B`
            (set `self.bAiming` false)
            (goto _label_11))))))
  (:`Completed`
    (goto _label_10 :!via `Reset`)))

(event `self.OnLanded`
  (params (Hit :type "HitResult Structure (by ref)"))
  (`self.StopWallRun`))

(event `EnhancedInput|/Game/FPSTutorial/Data/IA_Reload`
  (params (ActionValue :type Boolean) (ElapsedSeconds :type "Float (double-precision)") (TriggeredSeconds :type "Float (double-precision)") (InputAction :type "InputAction Object Reference" :default "/Game/FPSTutorial/Data/IA_Reload.IA_Reload"))
  (:`Triggered`
    (`/Engine/EditorBlueprintResources/StandardMacros.DoOnce` false :!label _label_12
      (:`Completed`
        (if (and (not (`self.bReloading`)) (< (`self.CurrentAmmo`) (`self.MagSize`)) (`self.bEquipped`))
          (set `self.bReloading` true)
          (`|PlayMontage` (`self.CharacterArms`) (select `int` (`self.EquipIndex`) :`0` "/Game/FPSTutorial/Art/Gun/Animations/AM_FP_Gun_Reload.AM_FP_Gun_Reload" :`1` "/Game/FPSTutorial/Art/Glock18/Animations/AM_FP_Glock_Reload.AM_FP_Glock_Reload" :!type "AnimMontage Object Reference")
            (:`then`
              (message `/Game/FPSTutorial/Core/BPI_Weapon.Reload` (`|GetArrayItem` (`self.EquippedWeapons`) (`self.EquipIndex`))))
            (:`OnBlendOut`
              (set `self.bReloading` false)))))))
  (:`Completed`
    (goto _label_12 :!via `Reset`)))

(event `EnhancedInput|/Game/FPSTutorial/Data/IA_Movement`
  (params (ActionValue :type "Vector2D Structure") (ElapsedSeconds :type "Float (double-precision)") (TriggeredSeconds :type "Float (double-precision)") (InputAction :type "InputAction Object Reference" :default "/Game/FPSTutorial/Data/IA_Movement.IA_Movement"))
  (bind (_x _y) (`KismetMathLibrary.BreakVector2D` (`self.KeebInput`)))
  (:`Triggered`
    (set `self.KeebInput` ActionValue :!label _label_13)
    (`self.AddMovementInput` (* (`self.GetActorForwardVector`) _y))
    (`self.AddMovementInput` (* (`self.GetActorRightVector`) _x)))
  (:`Completed`
    (goto _label_13)))

(event `Key|L`
  (params (Key :type "Key Structure"))
  (:`Pressed`
    (`/Engine/EditorBlueprintResources/StandardMacros.DoOnce` false :!label _label_14
      (:`Completed`
        (`KismetSystemLibrary.PrintString` "Attempting To Fuck The Sun")
        (message `/Game/FPSTutorial/Core/BPI_Interactable_Interface.FucktheSun` (`self.SunToFuck`)))))
  (:`Released`
    (goto _label_14 :!via `Reset`)))

(event `EnhancedInput|/Game/FPSTutorial/Data/IA_Interact`
  (params (ActionValue :type Boolean) (ElapsedSeconds :type "Float (double-precision)") (TriggeredSeconds :type "Float (double-precision)") (InputAction :type "InputAction Object Reference" :default "/Game/FPSTutorial/Data/IA_Interact.IA_Interact"))
  (:`Triggered`
    (`/Engine/EditorBlueprintResources/StandardMacros.DoOnce` false :!label _label_15
      (:`Completed`
        (message `/Game/FPSTutorial/Core/BPI_Interactable_Interface.Interact_Event` (`.HitActor` (`GameplayStatics.BreakHitResult` (`self.Interactable`)))))))
  (:`Completed`
    (goto _label_15 :!via `Reset`)))

(event `EnhancedInput|/Game/FPSTutorial/Data/IA_CameraLook`
  (params (ActionValue :type "Vector2D Structure") (ElapsedSeconds :type "Float (double-precision)") (TriggeredSeconds :type "Float (double-precision)") (InputAction :type "InputAction Object Reference" :default "/Game/FPSTutorial/Data/IA_CameraLook.IA_CameraLook"))
  (:`Triggered`
    (bind _output_get (set `self.MouseInput` ActionValue :!label _label_16))
    (bind (_x _y) (`KismetMathLibrary.BreakVector2D` _output_get))
    (`self.AddControllerPitchInput` (* _y -1.0))
    (`self.AddControllerYawInput` _x))
  (:`Completed`
    (goto _label_16)))

(event `HolsterToggle`
  (if (not (`self.bReloading`))
    (set `self.bEquipped` (not (`self.bEquipped`)))
    (message `/Game/FPSTutorial/Core/BPI_Weapon.Equip` (`|GetArrayItem` (`self.EquippedWeapons`) (`self.EquipIndex`)))
    (`|PlayMontage` (`self.CharacterArms`) (select `bool` (`self.bEquipped`) :`false` "/Game/FPSTutorial/Art/Gun/Animations/AM_FP_Gun_Holster.AM_FP_Gun_Holster" :`true` "/Game/FPSTutorial/Art/Gun/Animations/AM_FP_Gun_Equip.AM_FP_Gun_Equip" :!type "AnimMontage Object Reference"))))

(event `EnhancedInput|/Game/FPSTutorial/Data/IA_Sprint`
  (params (ActionValue :type Boolean) (ElapsedSeconds :type "Float (double-precision)") (TriggeredSeconds :type "Float (double-precision)") (InputAction :type "InputAction Object Reference" :default "/Game/FPSTutorial/Data/IA_Sprint.IA_Sprint"))
  (bind _charactermovement (`self.CharacterMovement`))
  (:`Triggered`
    (if (`NavMovementComponent.IsFalling` _charactermovement)
      _
      (elif (not (`self.bCrouching`))
        (set `CharacterMovementComponent.MaxWalkSpeed` (`self.RunningSpeed`) _charactermovement)
        (set `self.bSprinting` true)
        (bind (_direction _camera_fov) (`Timeline|FOVTimeline` :!label _label_17)
          (:`Update`
            (set `PlayerCameraManager.DefaultFOV` _camera_fov (`GameplayStatics.GetPlayerCameraManager` 0)))))))
  (:`Completed`
    (`self.StopRunning`)))

(event `EnableCamo`
  (bind _characterarms (`self.CharacterArms`))
  (bind _dynamiccamomat1 (`self.DynamicCamoMat1`))
  (bind _dynamiccamomat2 (`self.DynamicCamoMat2`))
  (`|ExecutionSequence`
    (:`then_0`
      (for _array_element (`self.EquippedWeapons`)
        (message `/Game/FPSTutorial/Core/BPI_Weapon.EnableCamo` _array_element)))
    (:`then_1`
      (`PrimitiveComponent.SetMaterial` _characterarms 1 _dynamiccamomat1)
      (`PrimitiveComponent.SetMaterial` _characterarms 0 _dynamiccamomat2)
      (bind (_direction _opacity) (`Timeline|CamoOpacity` :!via `PlayFromStart` :!label _label_18)
        (:`Update`
          (`MaterialInstanceDynamic.SetScalarParameterValue` _dynamiccamomat1 "Opacity" _opacity)
          (`MaterialInstanceDynamic.SetScalarParameterValue` _dynamiccamomat2 "Opacity" _opacity))))))

(event `StopRunning`
  (set `CharacterMovementComponent.MaxWalkSpeed` 600.0 (`self.CharacterMovement`))
  (set `self.bSprinting` false)
  (goto _label_17 :!via `Reverse`))

(event `DisableCamo`
  (bind _characterarms (`self.CharacterArms`))
  (`|ExecutionSequence`
    (:`then_0`
      (`|ExecutionSequence`
        (:`then_0`
          (goto _label_18 :!via `Reverse`))
        (:`then_1`
          (`PrimitiveComponent.SetMaterial` _characterarms 1 "/Game/FPSTutorial/Art/Mannequins/Materials/MI_Manny-Color-Player.MI_Manny-Color-Player")
          (`PrimitiveComponent.SetMaterial` _characterarms 0 "/Game/FPSTutorial/Art/Mannequins/Materials/MI_Mannequin-Color_Player.MI_Mannequin-Color_Player"))))
    (:`then_1`
      (for _array_element (`self.EquippedWeapons`)
        (message `/Game/FPSTutorial/Core/BPI_Weapon.DisableCamo` _array_element)))))

(event `EnhancedInput|/Game/FPSTutorial/Data/IA_Jump`
  (params (ActionValue :type Boolean) (ElapsedSeconds :type "Float (double-precision)") (TriggeredSeconds :type "Float (double-precision)") (InputAction :type "InputAction Object Reference" :default "/Game/FPSTutorial/Data/IA_Jump.IA_Jump"))
  (bind _iswallrunning (`self.IsWallRunning`))
  (:`Triggered`
    (if _iswallrunning
      (`self.StopWallRun`)
      (`self.LaunchCharacter` (+ (* (`MovementComponent.GetPlaneConstraintNormal` (`self.CharacterMovement`)) 700.0) (0.0 0.0 350.0)))
      (`|PlayMontage` (`self.CharacterArms`) (select `bool` (> (`self.WallRunDir`) 0.0) :`false` "/Game/FPSTutorial/Art/Gun/Animations/AM_FP_Gun_WallJump_R.AM_FP_Gun_WallJump_R" :`true` "/Game/FPSTutorial/Art/Gun/Animations/AM_FP_Gun_WallJump_L.AM_FP_Gun_WallJump_L" :!type "AnimMontage Object Reference") 2.0)
      (else
        (`self.Jump`)
        (if (not _iswallrunning)
          (`self.StopRunning`)))))
  (:`Completed`
    (`self.StopJumping`)))

(event `EnhancedInput|/Game/FPSTutorial/Data/IA_ScrollEquip`
  (params (ActionValue :type "Float (double-precision)") (ElapsedSeconds :type "Float (double-precision)") (TriggeredSeconds :type "Float (double-precision)") (InputAction :type "InputAction Object Reference" :default "/Game/FPSTutorial/Data/IA_ScrollEquip.IA_ScrollEquip"))
  (bind _equippedweapons (`self.EquippedWeapons`))
  (bind _editequipindex (`self.editEquipIndex`))
  (bind _output (`|GetArrayItem` _equippedweapons (`self.EquipIndex`)))
  (bind _returnvalue (- (`KismetArrayLibrary.Array_Length` (`self.EquippedWeapons`)) 1))
  (:`Triggered`
    (`/Engine/EditorBlueprintResources/StandardMacros.DoOnce` false :!label _label_19
      (:`Completed`
        (if (and (`self.bEquipped`) (not (`self.bReloading`)))
          (message `/Game/FPSTutorial/Core/BPI_Weapon.Holster` (`|GetArrayItem` (`self.EquippedWeapons`) (`self.EquipIndex`)))
          (`|PlayMontage` (`self.CharacterArms`) (select `int` (`self.EquipIndex`) :`0` "/Game/FPSTutorial/Art/Gun/Animations/AM_FP_Gun_Holster.AM_FP_Gun_Holster" :`1` "/Game/FPSTutorial/Art/Glock18/Animations/AM_FP_Glock_Holster.AM_FP_Glock_Holster" :!type "AnimMontage Object Reference")
            (:`then`
              (set `self.editEquipIndex` (+ ActionValue _editequipindex))
              (if (> _editequipindex _returnvalue)
                (set `self.editEquipIndex` 0)
                (elif (< _editequipindex 0)
                  (set `self.editEquipIndex` _returnvalue)
                  (else
                    (set `self.editEquipIndex` _editequipindex))))
              (`KismetSystemLibrary.Delay` 0.5)
              (set `self.EquipIndex` (`self.editEquipIndex`))
              (for _array_element _equippedweapons
                (`self.SetActorHiddenInGame` _array_element true))
              (`self.SetActorHiddenInGame` _output false)
              (`|PlayMontage` (`self.CharacterArms`) (select `int` (`self.EquipIndex`) :`0` "/Game/FPSTutorial/Art/Gun/Animations/AM_FP_Gun_Equip.AM_FP_Gun_Equip" :`1` "/Game/FPSTutorial/Art/Glock18/Animations/AM_FP_Glock_Equip.AM_FP_Glock_Equip" :!type "AnimMontage Object Reference")
                (:`then`
                  (message `/Game/FPSTutorial/Core/BPI_Weapon.Equip` _output)))))))))
  (:`Completed`
    (goto _label_19 :!via `Reset`)))

(event `EnhancedInput|/Game/FPSTutorial/Data/IA_Crouch`
  (params (ActionValue :type Boolean) (ElapsedSeconds :type "Float (double-precision)") (TriggeredSeconds :type "Float (double-precision)") (InputAction :type "InputAction Object Reference" :default "/Game/FPSTutorial/Data/IA_Crouch.IA_Crouch"))
  (:`Triggered`
    (`/Engine/EditorBlueprintResources/StandardMacros.DoOnce` false :!label _label_20
      (:`Completed`
        (if (`self.bHoldCrouch`)
          (`self.CustomCrouch`)
          (else
            (`/Engine/EditorBlueprintResources/StandardMacros.FlipFlop`
              (:`A`
                (`self.CustomCrouch`))
              (:`B`
                (`self.CustomUnCrouch`))))))))
  (:`Completed`
    (`|ExecutionSequence`
      (:`then_0`
        (if (`self.bHoldCrouch`)
          (`self.CustomUnCrouch`)))
      (:`then_1`
        (goto _label_20 :!via `Reset`)))))

(event `CustomCrouch`
  (set `self.bCrouching` true)
  (`self.StopRunning`)
  (set `CharacterMovementComponent.MaxWalkSpeed` 300.0 (`self.CharacterMovement`))
  (bind (_direction _capsule_half_height) (`Timeline|CrouchTimeline` :!label _label_21)
    (:`Update`
      (`CapsuleComponent.SetCapsuleHalfHeight` (`self.CapsuleComponent`) _capsule_half_height true))
    (:`Finished`
      (`/Engine/EditorBlueprintResources/StandardMacros.FlipFlop`
        (:`A`
          (`self.EnableCamo`))
        (:`B`
          (`self.DisableCamo`))))))

(event `CustomUnCrouch`
  (set `self.bCrouching` false)
  (set `CharacterMovementComponent.MaxWalkSpeed` 600.0 (`self.CharacterMovement`))
  (goto _label_21 :!via `Reverse`))

(fn `CheckForWall`
  (params (Hit :type "HitResult Structure"))
  (returns (`Hit Wall Info` :type "HitResult Structure") (IsWall :type Boolean))
  (bind _returnvalue (`KismetMathLibrary.Dot_VectorVector` (`.Normal` (`GameplayStatics.BreakHitResult` Hit)) (`self.GetActorRightVector`)))
  (set `self.WallRunDir` _returnvalue)
  (return Hit (> (`KismetMathLibrary.Abs` _returnvalue) 0.8)))

(fn `SpawnInventory`
  (for _array_element (`self.Inventory`)
    (bind _returnvalue (`|SpawnActorFromClass` _array_element (`KismetMathLibrary.MakeTransform` (0.0 0.0 0.0)) "Undefined" "MultiplyWithRoot" null null))
    (`KismetArrayLibrary.Array_Add` (`self.EquippedWeapons`) _returnvalue)
    (`self.K2_AttachToComponent` _returnvalue (`self.CharacterArms`) "ik_hand_gun" "KeepRelative" "KeepRelative" "KeepRelative" true)
    (`self.SetActorHiddenInGame` _returnvalue true))
  (`self.SetActorHiddenInGame` (`|GetArrayItem` (`self.EquippedWeapons`) (`self.EquipIndex`)) false))

(fn `StartWallRun`
  (params (PlaneNormal :type "Vector Structure"))
  (bind _charactermovement (`self.CharacterMovement`))
  (if (and (`NavMovementComponent.IsFalling` _charactermovement) (not (`self.IsWallRunning`)))
    (set `self.IsWallRunning` true)
    (`MovementComponent.SetPlaneConstraintEnabled` _charactermovement true)
    (`MovementComponent.SetPlaneConstraintNormal` _charactermovement PlaneNormal)
    (`self.StopJumping`)
    (set `CharacterMovementComponent.GravityScale` 0.4 _charactermovement)
    (if (not (`self.bSprinting`))
      (set `CharacterMovementComponent.MaxWalkSpeed` 1000.0 _charactermovement))))

(fn `StopWallRun`
  (bind _charactermovement (`self.CharacterMovement`))
  (set `self.IsWallRunning` false)
  (`MovementComponent.SetPlaneConstraintEnabled` _charactermovement false)
  (set `CharacterMovementComponent.GravityScale` 1.0 _charactermovement)
  (if (not true)
    (set `CharacterMovementComponent.MaxWalkSpeed` 600.0 _charactermovement)))

(fn `UserConstructionScript`)