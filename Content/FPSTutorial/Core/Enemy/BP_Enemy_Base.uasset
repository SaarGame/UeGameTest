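; Base enemy character for a shooter, exposing gun equipping, attacking, patrol route and movement speed functions, and mirroring the passive flag from its AI controller.
; Attack spawns a bullet at the head with mutual move-ignore, then signals attack end.
; Any damage reduces health and calls the controller's SetStateAsDead, even when non-lethal.
; At zero health the mesh ragdolls, the player's capsule ignores it, and its hidden weapon is replaced by a dropped dummy gun.
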(event `self.ReceiveBeginPlay`
  (set `self.CurrentHealth` (`KismetMathLibrary.Conv_IntToDouble` (`self.MaxHealth`)))
  (set `self.CurrentArmor` (`KismetMathLibrary.Conv_IntToDouble` (`self.MaxArmor`))))

(event `self.ReceiveTick`
  (params (DeltaSeconds :type "Float (single-precision)"))
  (bind _asaic_enemy_base (cast `/Game/FPSTutorial/Core/Enemy/AI/AIC_Enemy_Base` (`AIBlueprintHelperLibrary.GetAIController` self)))
  (set `self.IsPassive` (`/Game/FPSTutorial/Core/Enemy/AI/AIC_Enemy_Base.IsPassive` _asaic_enemy_base)))

(event `self.ReceiveAnyDamage`
  (params (Damage :type "Float (single-precision)") (DamageType :type "DamageType Object Reference") (InstigatedBy :type "Controller Object Reference") (DamageCauser :type "Actor Object Reference"))
  (bind _isdead (`self.IsDead`))
  (bind _currenthealth (`self.CurrentHealth`))
  (set `self.CurrentHealth` (- _currenthealth Damage))
  (set `self.IsDead` (<= _currenthealth 0.0))
  (bind _asaic_enemy_base (cast `/Game/FPSTutorial/Core/Enemy/AI/AIC_Enemy_Base` (`AIBlueprintHelperLibrary.GetAIController` self)))
  (`/Game/FPSTutorial/Core/Enemy/AI/AIC_Enemy_Base.SetStateAsDead` _asaic_enemy_base)
  (`|ExecutionSequence`
    (:`then_0`
      (`PrimitiveComponent.SetSimulatePhysics` (`self.Mesh`) _isdead)
      (`PrimitiveComponent.IgnoreActorWhenMoving` (`Character.CapsuleComponent` (`GameplayStatics.GetPlayerCharacter` 0)) self _isdead)
      (`self.SetActorHiddenInGame` (`self.EquippedWeapon`) _isdead))
    (:`then_1`
      (if _isdead
        (`/Engine/EditorBlueprintResources/StandardMacros.DoOnce` false
          (:`Completed`
            (bind _returnvalue (`|SpawnActorFromClass` "/Game/FPSTutorial/Core/Weapons/Gun/BP_DummyGun.BP_DummyGun_C" (`SceneComponent.GetSocketTransform` (`self.Mesh`) "ik_hand_gun" "RTS_World") "AdjustIfPossibleButAlwaysSpawn" "MultiplyWithRoot" null null))
            (`PrimitiveComponent.SetMaterial` (`/Game/FPSTutorial/Core/Weapons/Gun/BP_DummyGun.GunMesh` _returnvalue) 0 "/Game/FPSTutorial/Art/Gun/Materials/MI_Gun-Green.MI_Gun-Green")))))))

(event `Attack`
  (bind _returnvalue (`|SpawnActorFromClass` "/Game/FPSTutorial/Core/Weapons/Gun/BP_Bullet.BP_Bullet_C" (`SceneComponent.K2_GetComponentToWorld` (`self.Head`)) "Undefined" "MultiplyWithRoot" null null))
  (`PrimitiveComponent.IgnoreActorWhenMoving` (`/Game/FPSTutorial/Core/Weapons/Gun/BP_Bullet.SM_Gun_Bullet` _returnvalue) self true)
  (`PrimitiveComponent.IgnoreActorWhenMoving` (`self.CapsuleComponent`) _returnvalue true)
  (`self.OnAttackEnd`))

(event `EquipGun`
  (bind _mesh (`self.Mesh`))
  (bind _returnvalue (`|SpawnActorFromClass` "/Game/FPSTutorial/Core/BP_Gun-Green.BP_Gun-Green_C" (`SceneComponent.K2_GetComponentToWorld` _mesh) "Undefined" "MultiplyWithRoot" null null))
  (bind _output_get (set `self.EquippedWeapon` _returnvalue))
  (`self.K2_AttachToComponent` _output_get _mesh "ik_hand_gun" "SnapToTarget" "SnapToTarget" "SnapToTarget" true)
  (set `self.IsEquipped` true))

(fn `GetPatrolRoute`
  (returns (PatrolRoute :type "/Game/FPSTutorial/Core/Enemy/AI/BP_PatrolRoute Object Reference"))
  (return (`self.PatrolRoute`)))

(fn `SetMovementSpeed`
  (params (Speed :type "/Game/FPSTutorial/Core/Enemy/AI/Enums/E_MovementSpeed Enum" :default "NewEnumerator0"))
  (returns (SpeedValue :type "Float (double-precision)"))
  (bind _output_get (set `CharacterMovementComponent.MaxWalkSpeed` (select `/Game/FPSTutorial/Core/Enemy/AI/Enums/E_MovementSpeed` Speed :`NewEnumerator1` 230.0 :`NewEnumerator3` 500.0 :!type "Float (single-precision)") (`self.CharacterMovement`)))
  (return _output_get))

(fn `UserConstructionScript`)