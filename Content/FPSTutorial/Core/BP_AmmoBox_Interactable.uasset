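; Interactable ammo box that refills one ammo type for the player's BP_Character.
; On BeginPlay it reads the player's current count for its AmmoType from the AmmoTypes map and caches it as the maximum.
; InteractEvent writes that cached value back with a map Add, resetting the count to its starting amount rather than incrementing it.
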(event `self.ReceiveBeginPlay`
  (bind _asbp_character (cast `/Game/FPSTutorial/Core/Character/BP_Character` (`GameplayStatics.GetPlayerCharacter` 0)))
  (set `self.MaxAmmoOfType` (`BlueprintMapLibrary.Map_Find` (`/Game/FPSTutorial/Core/Character/BP_Character.AmmoTypes` _asbp_character) (`self.AmmoType`))))

(event `/Game/FPSTutorial/Core/BPI_Interactable_Interface.Interact_Event`
  (`BlueprintMapLibrary.Map_Add` (`/Game/FPSTutorial/Core/Character/BP_Character.AmmoTypes` (stale `self.ReceiveBeginPlay` _asbp_character)) (`self.AmmoType`) (`self.MaxAmmoOfType`)))

(fn `UserConstructionScript`)