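; Glock pistol weapon for the FPS player, handling firing, reloading, equip and holster sounds, and an active-camo effect.
; Shoot spawns a bullet from the camera plus an ejected casing; Reload drops an empty mag and refills only when reserves hold a full magazine.
; Reserve ammo lives in BP_Character's AmmoTypes map, with Tick mirroring ammo state to the character while EquipIndex is 1.
; Camo swaps in a dynamic material with timeline-driven opacity.
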(event `self.ReceiveBeginPlay`
  (`parent.ReceiveBeginPlay`)
  (bind _asbp_character (cast `/Game/FPSTutorial/Core/Character/BP_Character` (`GameplayStatics.GetPlayerCharacter` 0)))
  (set `self.LocalTotalAmmo` (`BlueprintMapLibrary.Map_Find` (`/Game/FPSTutorial/Core/Character/BP_Character.AmmoTypes` _asbp_character) (`self.AmmoType`)))
  (set `self.LocalCurrentAmmo` (`self.MagSize`)))

(event `self.ReceiveTick`
  (params (DeltaSeconds :type "Float (single-precision)"))
  (`parent.ReceiveTick` DeltaSeconds)
  (bind _asbp_character (cast `/Game/FPSTutorial/Core/Character/BP_Character` (`GameplayStatics.GetPlayerCharacter` 0)))
  (if (== (`/Game/FPSTutorial/Core/Character/BP_Character.EquipIndex` _asbp_character) 1)
    (set `self.LocalTotalAmmo` (`BlueprintMapLibrary.Map_Find` (`/Game/FPSTutorial/Core/Character/BP_Character.AmmoTypes` _asbp_character) (`self.AmmoType`)))
    (set `/Game/FPSTutorial/Core/Character/BP_Character.CurrentAmmo` (`self.LocalCurrentAmmo`) _asbp_character)
    (set `/Game/FPSTutorial/Core/Character/BP_Character.TotalAmmo` (`self.LocalTotalAmmo`) _asbp_character)
    (set `/Game/FPSTutorial/Core/Character/BP_Character.MagSize` (`self.MagSize`) _asbp_character)
    (set `/Game/FPSTutorial/Core/Character/BP_Character.CurrentAmmoType` (`self.AmmoType`) _asbp_character)))

(event `/Game/FPSTutorial/Core/BPI_Weapon.Shoot`
  (bind _sk_gun (`self.SK_Gun`))
  (bind _firesoundvariance (`self.FireSoundVariance`))
  (bind _asbp_character (cast `/Game/FPSTutorial/Core/Character/BP_Character` (`GameplayStatics.GetPlayerCharacter` 0)))
  (bind _returnvalue (`|SpawnActorFromClass` "/Game/FPSTutorial/Core/Weapons/Glock/BP_Glock_Bullet.BP_Glock_Bullet_C" (`SceneComponent.K2_GetComponentToWorld` (`/Game/FPSTutorial/Core/Character/BP_Character.Camera` _asbp_character)) "AlwaysSpawn" "MultiplyWithRoot" null null))
  (`PrimitiveComponent.IgnoreActorWhenMoving` (`/Game/FPSTutorial/Core/Weapons/Glock/BP_Glock_Bullet.SM_Gun_Bullet` _returnvalue) _asbp_character true)
  (`PrimitiveComponent.IgnoreActorWhenMoving` (`Character.CapsuleComponent` _asbp_character) _returnvalue true)
  (set `self.LocalCurrentAmmo` (- (`self.LocalCurrentAmmo`) 1))
  (`|PlayMontage` _sk_gun "/Game/FPSTutorial/Art/Glock18/Animations/AM_WEP_Glock_Fire.AM_WEP_Glock_Fire" 2.0
    (:`then`
      (bind _returnvalue_2 (`|SpawnActorFromClass` "/Game/FPSTutorial/Core/Weapons/Glock/BP_Glock_Casing.BP_Glock_Casing_C" (`SceneComponent.GetSocketTransform` _sk_gun "SOCKET_Eject" "RTS_World") "AlwaysSpawn" "MultiplyWithRoot" null null))
      (`PrimitiveComponent.IgnoreActorWhenMoving` (`/Game/FPSTutorial/Core/Weapons/Glock/BP_Glock_Casing.SM_GunCasing` _returnvalue_2) (`GameplayStatics.GetPlayerCharacter` 0) false)
      (`GameplayStatics.PlaySound2D` (`|GetArrayItem` _firesoundvariance (`KismetMathLibrary.RandomInteger` (- (`KismetArrayLibrary.Array_Length` _firesoundvariance) 1))) 1.0 1.0 0.0 null null))))

(event `/Game/FPSTutorial/Core/BPI_Weapon.Reload`
  (bind _returnvalue (== (`self.LocalCurrentAmmo`) 0))
  (bind _asbp_character (cast `/Game/FPSTutorial/Core/Character/BP_Character` (`GameplayStatics.GetPlayerCharacter` 0)))
  (`|PlayMontage` (`self.SK_Gun`) "/Game/FPSTutorial/Art/Glock18/Animations/AM_WEP_Glock_Reload.AM_WEP_Glock_Reload"
    (:`then`
      (`KismetSystemLibrary.Delay` 0.8)
      (`GameplayStatics.PlaySound2D` "/Game/FPSTutorial/Art/Gun/Sounds/Mag_Takeout1.Mag_Takeout1" 1.0 1.0 0.0 null null)
      (bind _returnvalue_2 (`|SpawnActorFromClass` "/Game/FPSTutorial/Core/Weapons/Glock/BP_Glock_EmptyMag.BP_Glock_EmptyMag_C" (`KismetMathLibrary.MakeTransform` (- (.location (`SceneComponent.K2_GetComponentToWorld` (`/Game/FPSTutorial/Core/Character/BP_Character.Camera` _asbp_character))) (0.0 8.0 50.0)) (.rotation (`SceneComponent.K2_GetComponentToWorld` (`/Game/FPSTutorial/Core/Character/BP_Character.Camera` _asbp_character))) (.scale (`SceneComponent.K2_GetComponentToWorld` (`/Game/FPSTutorial/Core/Character/BP_Character.Camera` _asbp_character)))) "Undefined" "MultiplyWithRoot" null null))
      (`PrimitiveComponent.IgnoreActorWhenMoving` (`/Game/FPSTutorial/Core/Weapons/Glock/BP_Glock_EmptyMag.Mag` _returnvalue_2) _asbp_character true)
      (`PrimitiveComponent.IgnoreActorWhenMoving` (`Character.CapsuleComponent` _asbp_character) _returnvalue_2 true)
      (`KismetSystemLibrary.Delay` (`self.ReloadDelay`))
      (`GameplayStatics.PlaySound2D` "/Game/FPSTutorial/Art/Glock18/Sounds/Mag_Insert1.Mag_Insert1" 1.0 1.0 0.0 null null)
      (if _returnvalue
        (`GameplayStatics.PlaySound2D` "/Game/FPSTutorial/Art/Glock18/Sounds/Bolt_Release1.Bolt_Release1" 1.0 1.0 0.0 null null))
      (if (>= (`self.LocalTotalAmmo`) (`self.MagSize`))
        (if _returnvalue
          (set `self.AmmoToRemove` (`self.MagSize`))
          (else
            (set `self.AmmoToRemove` (- (`self.MagSize`) (`self.LocalCurrentAmmo`)))))
        (set `self.LocalCurrentAmmo` (+ (`self.LocalCurrentAmmo`) (`self.AmmoToRemove`)))
        (set `self.LocalTotalAmmo` (- (`self.LocalTotalAmmo`) (`self.AmmoToRemove`)))
        (bind _asbp_character_2 (cast `/Game/FPSTutorial/Core/Character/BP_Character` (`GameplayStatics.GetPlayerCharacter` 0)))
        (`BlueprintMapLibrary.Map_Add` (`/Game/FPSTutorial/Core/Character/BP_Character.AmmoTypes` _asbp_character_2) (`self.AmmoType`) (`self.LocalTotalAmmo`))))))

(event `/Game/FPSTutorial/Core/BPI_Weapon.Equip`
  (`GameplayStatics.PlaySound2D` "/Game/FPSTutorial/Art/Glock18/Sounds/Grab1.Grab1" 1.0 1.0 0.0 null null))

(event `/Game/FPSTutorial/Core/BPI_Weapon.Holster`
  (`GameplayStatics.PlaySound2D` "/Game/FPSTutorial/Art/Gun/Sounds/Holster1.Holster1" 1.0 1.0 0.0 null null))

(event `/Game/FPSTutorial/Core/BPI_Weapon.InitCamo`
  (bind _returnvalue (`KismetMaterialLibrary.CreateDynamicMaterialInstance` "/Game/FPSTutorial/Art/Glock18/Materials/M_Glock18_ActiveCamo.M_Glock18_ActiveCamo"))
  (set `self.DynamicCamoMat` _returnvalue))

(event `/Game/FPSTutorial/Core/BPI_Weapon.EnableCamo`
  (bind _sk_gun (`self.SK_Gun`))
  (bind _mag (`self.Mag`))
  (bind _dynamiccamomat (`self.DynamicCamoMat`))
  (`PrimitiveComponent.SetMaterial` _sk_gun 0 _dynamiccamomat)
  (`PrimitiveComponent.SetMaterial` _sk_gun 1 _dynamiccamomat)
  (`PrimitiveComponent.SetMaterial` _mag 0 _dynamiccamomat)
  (`PrimitiveComponent.SetMaterial` _mag 1 _dynamiccamomat)
  (bind (_direction _opacity) (`Timeline|CamoOpacity` :!via `PlayFromStart` :!label _label)
    (:`Update`
      (`MaterialInstanceDynamic.SetScalarParameterValue` _dynamiccamomat "Opacity" _opacity))))

(event `/Game/FPSTutorial/Core/BPI_Weapon.DisableCamo`
  (bind _sk_gun (`self.SK_Gun`))
  (bind _mag (`self.Mag`))
  (`|ExecutionSequence`
    (:`then_0`
      (goto _label :!via `Reverse`))
    (:`then_1`
      (`PrimitiveComponent.SetMaterial` _sk_gun 0 "/Game/FPSTutorial/Art/Glock18/Materials/MI_Glock18.MI_Glock18")
      (`PrimitiveComponent.SetMaterial` _sk_gun 1 "/Game/FPSTutorial/Art/Glock18/Materials/MI_Glock18.MI_Glock18")
      (`PrimitiveComponent.SetMaterial` _mag 0 "/Game/FPSTutorial/Art/Glock18/Materials/MI_Glock18.MI_Glock18")
      (`PrimitiveComponent.SetMaterial` _mag 1 "/Game/FPSTutorial/Art/Glock18/Materials/MI_Glock18.MI_Glock18"))))

(fn `IsEmpty`
  (returns (Empty :type Boolean))
  (return false))

(fn `UserConstructionScript`
  (`parent.UserConstructionScript`))