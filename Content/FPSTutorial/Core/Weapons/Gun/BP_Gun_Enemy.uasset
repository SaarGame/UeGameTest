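; BP_Gun_Enemy is a gun Blueprint named for enemies, though its ammo logic reads and writes the player's BP_Character.
; Tick mirrors magazine and reserve ammo to the player while EquipIndex is 0.
; Reload times montage, sounds and a dropped magazine with delays, then refills only when reserves cover a full magazine.
; Shoot only prints its owner's name, leaving the bullet, casing and fire-montage logic disconnected.
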(event `self.ReceiveBeginPlay`
  (`parent.ReceiveBeginPlay`)
  (bind _asbp_character (cast `/Game/FPSTutorial/Core/Character/BP_Character` (`GameplayStatics.GetPlayerCharacter` 0)))
  (set `self.LocalTotalAmmo` (`BlueprintMapLibrary.Map_Find` (`/Game/FPSTutorial/Core/Character/BP_Character.AmmoTypes` _asbp_character) (`self.AmmoType`)))
  (set `self.LocalCurrentAmmo` (`self.MagSize`)))

(event `self.ReceiveTick`
  (params (DeltaSeconds :type "Float (single-precision)"))
  (`parent.ReceiveTick` DeltaSeconds)
  (bind _asbp_character (cast `/Game/FPSTutorial/Core/Character/BP_Character` (`GameplayStatics.GetPlayerCharacter` 0)))
  (if (== (`/Game/FPSTutorial/Core/Character/BP_Character.EquipIndex` _asbp_character) 0)
    (set `self.LocalTotalAmmo` (`BlueprintMapLibrary.Map_Find` (`/Game/FPSTutorial/Core/Character/BP_Character.AmmoTypes` _asbp_character) (`self.AmmoType`)))
    (set `/Game/FPSTutorial/Core/Character/BP_Character.CurrentAmmo` (`self.LocalCurrentAmmo`) _asbp_character)
    (set `/Game/FPSTutorial/Core/Character/BP_Character.TotalAmmo` (`self.LocalTotalAmmo`) _asbp_character)
    (set `/Game/FPSTutorial/Core/Character/BP_Character.MagSize` (`self.MagSize`) _asbp_character)
    (set `/Game/FPSTutorial/Core/Character/BP_Character.CurrentAmmoType` (`self.AmmoType`) _asbp_character)))

(event `self.Shoot`
  (`KismetSystemLibrary.PrintString` (`KismetSystemLibrary.GetDisplayName` (`self.GetOwner`))))

(event `self.Reload`
  (bind _returnvalue (`GameplayStatics.GetPlayerCharacter` 0))
  (bind _asbp_character (cast `/Game/FPSTutorial/Core/Character/BP_Character` _returnvalue))
  (`|PlayMontage` (`self.SK_Gun`) "/Game/FPSTutorial/Art/Gun/Animations/AM_FP_WEP_Gun_Reload.AM_FP_WEP_Gun_Reload"
    (:`then`
      (`KismetSystemLibrary.Delay` 0.4)
      (`GameplayStatics.PlaySound2D` "/Game/FPSTutorial/Art/Gun/Sounds/Mag_Takeout1.Mag_Takeout1" 1.0 1.0 0.0 null null)
      (bind _returnvalue_2 (`|SpawnActorFromClass` "/Game/FPSTutorial/Core/Weapons/Gun/BP_Gun_EmptyMag.BP_Gun_EmptyMag_C" (`KismetMathLibrary.MakeTransform` (- (.location (`SceneComponent.K2_GetComponentToWorld` (`/Game/FPSTutorial/Core/Character/BP_Character.Camera` _asbp_character))) (0.0 8.0 50.0)) (.rotation (`SceneComponent.K2_GetComponentToWorld` (`/Game/FPSTutorial/Core/Character/BP_Character.Camera` _asbp_character))) (.scale (`SceneComponent.K2_GetComponentToWorld` (`/Game/FPSTutorial/Core/Character/BP_Character.Camera` _asbp_character)))) "Undefined" "MultiplyWithRoot" null null))
      (`PrimitiveComponent.IgnoreActorWhenMoving` (`/Game/FPSTutorial/Core/Weapons/Gun/BP_Gun_EmptyMag.Mag` _returnvalue_2) _returnvalue true)
      (`PrimitiveComponent.IgnoreActorWhenMoving` (`Character.CapsuleComponent` _returnvalue) _returnvalue_2 true)
      (`KismetSystemLibrary.Delay` 1.5)
      (`GameplayStatics.PlaySound2D` "/Game/FPSTutorial/Art/Gun/Sounds/Mag_Insert1.Mag_Insert1" 1.0 1.0 0.0 null null)
      (`KismetSystemLibrary.Delay` (`self.ReloadDelay`))
      (if (>= (`self.LocalTotalAmmo`) (`self.MagSize`))
        (if (== (`self.LocalCurrentAmmo`) 0)
          (set `self.AmmoToRemove` (`self.MagSize`))
          (else
            (set `self.AmmoToRemove` (- (`self.MagSize`) (`self.LocalCurrentAmmo`)))))
        (set `self.LocalCurrentAmmo` (+ (`self.LocalCurrentAmmo`) (`self.AmmoToRemove`)))
        (set `self.LocalTotalAmmo` (- (`self.LocalTotalAmmo`) (`self.AmmoToRemove`)))
        (bind _asbp_character_2 (cast `/Game/FPSTutorial/Core/Character/BP_Character` (`GameplayStatics.GetPlayerCharacter` 0)))
        (`BlueprintMapLibrary.Map_Add` (`/Game/FPSTutorial/Core/Character/BP_Character.AmmoTypes` _asbp_character_2) (`self.AmmoType`) (`self.LocalTotalAmmo`))
        (`KismetSystemLibrary.Delay` 0.4)
        (`GameplayStatics.PlaySound2D` "/Game/FPSTutorial/Art/Gun/Sounds/Foregrip_Grab1.Foregrip_Grab1" 1.0 1.0 0.0 null null)))))

(event `self.Holster`
  (`GameplayStatics.PlaySound2D` "/Game/FPSTutorial/Art/Gun/Sounds/Holster1.Holster1" 1.0 1.0 0.0 null null))

(event `self.Equip`
  (`GameplayStatics.PlaySound2D` "/Game/FPSTutorial/Art/Gun/Sounds/Grab2.Grab2" 1.0 1.0 0.0 null null))

(fn `UserConstructionScript`
  (`parent.UserConstructionScript`))