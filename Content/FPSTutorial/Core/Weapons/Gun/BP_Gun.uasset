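; BP_Gun is the player's first-person gun, handling firing, reloading, equip sounds and an active camo material.
; While equip index is 0, Tick reads reserve ammo from BP_Character's AmmoTypes map and pushes ammo state to the character.
; Shoot spawns camera-aimed bullets and ejected casings and reports noise.
; Reload drops an empty mag, then refills after timed delays only if reserve holds at least a full magazine.
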(event `self.ReceiveBeginPlay`
  (`parent.ReceiveBeginPlay`)
  (bind _asbp_character (cast `/Game/FPSTutorial/Core/Character/BP_Character` (`GameplayStatics.GetPlayerCharacter` 0)))
  (set `self.LocalTotalAmmo` (`BlueprintMapLibrary.Map_Find` (`/Game/FPSTutorial/Core/Character/BP_Character.AmmoTypes` _asbp_character) (`self.AmmoType`)))
  (set `self.LocalCurrentAmmo` (`self.MagSize`)))

(event `self.ReceiveTick`
  (params (DeltaSeconds :type "Float (single-precision)"))
  (`parent.ReceiveTick` DeltaSeconds)
  (bind _asbp_character (cast `/Game/FPSTutorial/Core/Character/BP_Character` (`GameplayStatics.GetPlayerCharacter` 0)))
  (if (== (`/Game/FPSTutorial/Core/Character/BP_Character.EquipIndex` _asbp_character) 0)
    (set `self.LocalTotalAmmo` (`BlueprintMapLibrary.Map_Find` (`/Game/FPSTutorial/Core/Character/BP_Character.AmmoTypes` _asbp_character) (`self.AmmoType`)))
    (set `/Game/FPSTutorial/Core/Character/BP_Character.CurrentAmmo` (`self.LocalCurrentAmmo`) _asbp_character)
    (set `/Game/FPSTutorial/Core/Character/BP_Character.TotalAmmo` (`self.LocalTotalAmmo`) _asbp_character)
    (set `/Game/FPSTutorial/Core/Character/BP_Character.MagSize` (`self.MagSize`) _asbp_character)
    (set `/Game/FPSTutorial/Core/Character/BP_Character.CurrentAmmoType` (`self.AmmoType`) _asbp_character)))

(event `/Game/FPSTutorial/Core/BPI_Weapon.Shoot`
  (bind _returnvalue (`GameplayStatics.GetPlayerCharacter` 0))
  (bind _firesoundvariance (`self.FireSoundVariance`))
  (bind _sk_gun (`self.SK_Gun`))
  (bind _asbp_character (cast `/Game/FPSTutorial/Core/Character/BP_Character` (`GameplayStatics.GetPlayerCharacter` 0)))
  (bind _returnvalue_2 (`|SpawnActorFromClass` "/Game/FPSTutorial/Core/Weapons/Gun/BP_Bullet.BP_Bullet_C" (`SceneComponent.K2_GetComponentToWorld` (`/Game/FPSTutorial/Core/Character/BP_Character.Camera` _asbp_character)) "AlwaysSpawn" "MultiplyWithRoot" null null))
  (`PrimitiveComponent.IgnoreActorWhenMoving` (`/Game/FPSTutorial/Core/Weapons/Gun/BP_Bullet.SM_Gun_Bullet` _returnvalue_2) _asbp_character true)
  (`PrimitiveComponent.IgnoreActorWhenMoving` (`Character.CapsuleComponent` _asbp_character) _returnvalue_2 true)
  (set `self.LocalCurrentAmmo` (- (`self.LocalCurrentAmmo`) 1))
  (`|PlayMontage` _sk_gun "/Game/FPSTutorial/Art/Gun/Animations/AM_FP_WEP_Gun_Fire.AM_FP_WEP_Gun_Fire"
    (:`then`
      (bind _returnvalue_3 (`|SpawnActorFromClass` "/Game/FPSTutorial/Core/Weapons/Gun/BP_Casing.BP_Casing_C" (`SceneComponent.GetSocketTransform` _sk_gun "SOCKET_Eject" "RTS_World") "AlwaysSpawn" "MultiplyWithRoot" null null))
      (`PrimitiveComponent.IgnoreActorWhenMoving` (`/Game/FPSTutorial/Core/Weapons/Gun/BP_Casing.SM_GunCasing` _returnvalue_3) (`GameplayStatics.GetPlayerCharacter` 0) false)
      (`GameplayStatics.PlaySound2D` (`|GetArrayItem` _firesoundvariance (`KismetMathLibrary.RandomInteger` (- (`KismetArrayLibrary.Array_Length` _firesoundvariance) 1))) 1.0 1.0 0.0 null null)
      (`AISense_Hearing.ReportNoiseEvent` (`self.K2_GetActorLocation` _returnvalue) 1.0 _returnvalue))))

(event `/Game/FPSTutorial/Core/BPI_Weapon.Reload`
  (bind _returnvalue (`GameplayStatics.GetPlayerCharacter` 0))
  (bind _asbp_character (cast `/Game/FPSTutorial/Core/Character/BP_Character` _returnvalue))
  (`|PlayMontage` (`self.SK_Gun`) "/Game/FPSTutorial/Art/Gun/Animations/AM_FP_WEP_Gun_Reload.AM_FP_WEP_Gun_Reload"
    (:`then`
      (`KismetSystemLibrary.Delay` 0.4)
      (`GameplayStatics.PlaySound2D` "/Game/FPSTutorial/Art/Gun/Sounds/Mag_Takeout1.Mag_Takeout1" 1.0 1.0 0.0 null null)
      (bind _returnvalue_2 (`|SpawnActorFromClass` "/Game/FPSTutorial/Core/Weapons/Gun/BP_Gun_EmptyMag.BP_Gun_EmptyMag_C" (`KismetMathLibrary.MakeTransform` (- (.location (`SceneComponent.K2_GetComponentToWorld` (`/Game/FPSTutorial/Core/Character/BP_Character.Camera` _asbp_character))) (0.0 8.0 50.0)) (.rotation (`SceneComponent.K2_GetComponentToWorld` (`/Game/FPSTutorial/Core/Character/BP_Character.Camera` _asbp_character))) (.scale (`SceneComponent.K2_GetComponentToWorld` (`/Game/FPSTutorial/Core/Character/BP_Character.Camera` _asbp_character)))) "Undefined" "MultiplyWithRoot" null null))
      (`PrimitiveComponent.IgnoreActorWhenMoving` (`/Game/FPSTutorial/Core/Weapons/Gun/BP_Gun_EmptyMag.Mag` _returnvalue_2) _returnvalue true)
      (`PrimitiveComponent.IgnoreActorWhenMoving` (`Character.CapsuleComponent` _returnvalue) _returnvalue_2 true)
      (`KismetSystemLibrary.Delay` 1.5)
      (`GameplayStatics.PlaySound2D` "/Game/FPSTutorial/Art/Gun/Sounds/Mag_Insert1.Mag_Insert1" 1.0 1.0 0.0 null null)
      (`KismetSystemLibrary.Delay` (`self.ReloadDelay`))
      (if (>= (`self.LocalTotalAmmo`) (`self.MagSize`))
        (if (== (`self.LocalCurrentAmmo`) 0)
          (set `self.AmmoToRemove` (`self.MagSize`))
          (else
            (set `self.AmmoToRemove` (- (`self.MagSize`) (`self.LocalCurrentAmmo`)))))
        (set `self.LocalCurrentAmmo` (+ (`self.LocalCurrentAmmo`) (`self.AmmoToRemove`)))
        (set `self.LocalTotalAmmo` (- (`self.LocalTotalAmmo`) (`self.AmmoToRemove`)))
        (bind _asbp_character_2 (cast `/Game/FPSTutorial/Core/Character/BP_Character` (`GameplayStatics.GetPlayerCharacter` 0)))
        (`BlueprintMapLibrary.Map_Add` (`/Game/FPSTutorial/Core/Character/BP_Character.AmmoTypes` _asbp_character_2) (`self.AmmoType`) (`self.LocalTotalAmmo`))
        (`KismetSystemLibrary.Delay` 0.4)
        (`GameplayStatics.PlaySound2D` "/Game/FPSTutorial/Art/Gun/Sounds/Foregrip_Grab1.Foregrip_Grab1" 1.0 1.0 0.0 null null)))))

(event `/Game/FPSTutorial/Core/BPI_Weapon.Holster`
  (`GameplayStatics.PlaySound2D` "/Game/FPSTutorial/Art/Gun/Sounds/Holster1.Holster1" 1.0 1.0 0.0 null null))

(event `/Game/FPSTutorial/Core/BPI_Weapon.Equip`
  (`GameplayStatics.PlaySound2D` "/Game/FPSTutorial/Art/Gun/Sounds/Grab2.Grab2" 1.0 1.0 0.0 null null))

(event `/Game/FPSTutorial/Core/BPI_Weapon.InitCamo`
  (bind _returnvalue (`KismetMaterialLibrary.CreateDynamicMaterialInstance` "/Game/FPSTutorial/Art/Gun/Materials/M_Gun_ActiveCamo.M_Gun_ActiveCamo"))
  (set `self.DynamicCamoMat` _returnvalue))

(event `/Game/FPSTutorial/Core/BPI_Weapon.EnableCamo`
  (bind _dynamiccamomat (`self.DynamicCamoMat`))
  (`PrimitiveComponent.SetMaterial` (`self.SK_Gun`) 0 _dynamiccamomat)
  (`PrimitiveComponent.SetMaterial` (`self.Mag`) 0 _dynamiccamomat)
  (bind (_direction _opacity) (`Timeline|CamoOpacity` :!via `PlayFromStart` :!label _label)
    (:`Update`
      (`MaterialInstanceDynamic.SetScalarParameterValue` _dynamiccamomat "Opacity" _opacity))))

(event `/Game/FPSTutorial/Core/BPI_Weapon.DisableCamo`
  (`|ExecutionSequence`
    (:`then_0`
      (goto _label :!via `Reverse`))
    (:`then_1`
      (`PrimitiveComponent.SetMaterial` (`self.SK_Gun`) 0 "/Game/FPSTutorial/Art/Gun/Materials/MI_Gun.MI_Gun")
      (`PrimitiveComponent.SetMaterial` (`self.Mag`) 0 "/Game/FPSTutorial/Art/Gun/Materials/MI_Gun.MI_Gun"))))

(fn `UserConstructionScript`
  (`parent.UserConstructionScript`))