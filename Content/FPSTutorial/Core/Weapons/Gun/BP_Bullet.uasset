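; BP_Bullet is a gun projectile that reacts to its first hit.
; On mesh hit, a DoOnce spawns a small explosion effect and triggers a spawned FS_MasterField_Bullet field actor.
; It then reports an AI damage event credited to the player and pushes physics-simulating components with a velocity-scaled impulse.
; The ApplyDamage node is disconnected, so the bullet only reports damage without applying it.
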(event `self.SM_Gun_Bullet.OnComponentHit`
  (params (HitComponent :type "PrimitiveComponent Object Reference") (OtherActor :type "Actor Object Reference") (OtherComp :type "PrimitiveComponent Object Reference") (NormalImpulse :type "Vector Structure") (Hit :type "HitResult Structure (by ref)"))
  (bind _returnvalue (`GameplayStatics.GetPlayerCharacter` 0))
  (set `self.HitActor` OtherActor)
  (`/Engine/EditorBlueprintResources/StandardMacros.DoOnce` false
    (:`Completed`
      (`GameplayStatics.SpawnEmitterAtLocation` "/Game/StarterContent/Particles/P_Explosion.P_Explosion" (`self.K2_GetActorLocation`) (struct) (0.3 0.3 0.3))
      (bind _returnvalue_2 (`|SpawnActorFromClass` "/Game/FPSTutorial/Core/FS_MasterField_Bullet.FS_MasterField_Bullet_C" (`self.GetTransform`) "AlwaysSpawn" "MultiplyWithRoot" null null))
      (set `self.Field` _returnvalue_2)
      (`/Engine/EditorResources/FieldNodes/FS_MasterField.CE_Trigger` (`self.Field`))
      (`AISense_Damage.ReportDamageEvent` (`self.HitActor`) _returnvalue 10.0 (`self.K2_GetActorLocation` _returnvalue))
      (if (`SceneComponent.IsSimulatingPhysics` OtherComp "None")
        (`PrimitiveComponent.AddImpulseAtLocation` OtherComp (* (`self.GetVelocity`) (7.0 7.0 7.0)) (`self.K2_GetActorLocation`) "None")))))

(fn `UserConstructionScript`)