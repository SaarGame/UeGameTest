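; Example weapon scope that uses a SceneCaptureComponent2D and swaps the material on the scope mesh's render slot.
; BeginPlay hides the scope from its own capture and sets the capture tick interval if player pawn 0 is locally controlled.
; Aim-in enables the capture, applies the active render material and ticks faster.
; Aim-out clears that material, hides the capture and throttles its tick to save work while idle.
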(event `self.ReceiveBeginPlay`
  (if (`Pawn.IsLocallyControlled` (`GameplayStatics.GetPlayerPawn` 0))
    (`ActorComponent.SetComponentTickInterval` (`self.SceneCaptureComponent2D`) 0.04)
    (`KismetArrayLibrary.Array_AddUnique` (`SceneCaptureComponent.HiddenActors` (`self.SceneCaptureComponent2D`)) self)))

(event `/Game/ProceduralFramework/Extras/Blueprints/ScopeExample/BPI_Scopes.Scope Aim In`
  ;[0.006622 0.01374 0.01562] Activate the scope.
  (set `SceneCaptureComponent.bCaptureOnMovement` true (`self.SceneCaptureComponent2D`))
  (`SceneComponent.SetVisibility` (`self.SceneCaptureComponent2D`) true false)
  (`PrimitiveComponent.SetMaterialByName` (`self.Scope`) (`self.Render Slot Name`) (`self.Render Slot Active`))
  (`ActorComponent.SetComponentTickInterval` (`self.SceneCaptureComponent2D`) 0.02))

(event `/Game/ProceduralFramework/Extras/Blueprints/ScopeExample/BPI_Scopes.Scope Aim Out`
  ;[0.07292 0.03794 0.0394] Deactivate the scope.
  (set `SceneCaptureComponent.bCaptureOnMovement` false (`self.SceneCaptureComponent2D`))
  (`SceneComponent.SetVisibility` (`self.SceneCaptureComponent2D`) false false)
  (`PrimitiveComponent.SetMaterialByName` (`self.Scope`) (`self.Render Slot Name`) null)
  (`ActorComponent.SetComponentTickInterval` (`self.SceneCaptureComponent2D`) 5.0))

(fn `UserConstructionScript`)