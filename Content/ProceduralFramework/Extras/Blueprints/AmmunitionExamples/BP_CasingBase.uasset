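; Base Blueprint for ejected ammunition casings that tumble under physics and play impact sounds.
; INITCasing enables physics and adds randomized linear and angular velocity along the ejection transform's up and right axes.
; Hits above an impulse threshold call SpawnSound, which scales volume by impact strength and plays a random attenuated sound, or prints the surface when Debug is set.
; Only Concrete sounds are wired; Wood, Metal and Grass calls never run.
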(event `INIT Casing`
  (params (EjectionTransform :type "Transform Structure (by ref)"))
  (bind (_yawimpulserot_x _yawimpulserot_y) (`KismetMathLibrary.BreakVector2D` (`self.YawImpulseRot`)))
  (bind (_pitchimpulserot_x _pitchimpulserot_y) (`KismetMathLibrary.BreakVector2D` (`self.PitchImpulseRot`)))
  (bind (_ximpulseloc_x _ximpulseloc_y) (`KismetMathLibrary.BreakVector2D` (`self.XImpulseLoc`)))
  (bind (_yimpulseloc_x _yimpulseloc_y) (`KismetMathLibrary.BreakVector2D` (`self.YImpulseLoc`)))
  (bind _rotation (.rotation (`self.Ejection Transform`)))
  (bind _rotation_2 (.rotation (`self.Ejection Transform`)))
  (set `self.Ejection Transform` EjectionTransform)
  ;[0.02083 0.02083 0.02083] Simulate Physics
  (`PrimitiveComponent.SetSimulatePhysics` (`self.Casing`) true)
  ;[0.01042 0.01042 0.01042] Add Rotation
  (`PrimitiveComponent.SetPhysicsAngularVelocityInDegrees` (`self.Casing`) (+ (* (`KismetMathLibrary.GetUpVector` _rotation) (`KismetMathLibrary.RandomFloatInRange` _pitchimpulserot_x _pitchimpulserot_y)) (* (`KismetMathLibrary.GetRightVector` _rotation) (`KismetMathLibrary.RandomFloatInRange` _yawimpulserot_x _yawimpulserot_y))) true "None")
  (`PrimitiveComponent.SetAllPhysicsLinearVelocity` (`self.Casing`) (+ (* (`KismetMathLibrary.GetUpVector` _rotation_2) (`KismetMathLibrary.RandomFloatInRange` _yimpulseloc_x _yimpulseloc_y)) (* (`KismetMathLibrary.GetRightVector` _rotation_2) (`KismetMathLibrary.RandomFloatInRange` _ximpulseloc_x _ximpulseloc_y))) true))

(event `self.Casing.OnComponentHit`
  (params (HitComponent :type "PrimitiveComponent Object Reference") (OtherActor :type "Actor Object Reference") (OtherComp :type "PrimitiveComponent Object Reference") (NormalImpulse :type "Vector Structure") (Hit :type "HitResult Structure (by ref)"))
  (bind _returnvalue (`KismetMathLibrary.VSize` NormalImpulse))
  (bind (_bblockinghit _binitialoverlap _time _distance _location _impactpoint _normal _impactnormal _physmat) (`GameplayStatics.BreakHitResult` Hit))
  ;[0 0 0] ON IMPACT
  (if (> _returnvalue 40.0)
    (`self.Spawn Sound` (`PhysicalMaterial.SurfaceType` _physmat) (`KismetMathLibrary.MapRangeClamped` _returnvalue 300.0 800.0 0.2 1.0) _impactpoint)))

(event `CasingSound`
  (params (VolumeMultiplier :type "Float (single-precision)") (Location :type "Vector Structure") (RandomSound :type "Array of SoundBase Object Reference"))
  ;[0 0 0] ON IMPACT
  (`GameplayStatics.SpawnSoundAtLocation` (`KismetArrayLibrary.Array_Random` RandomSound) Location (struct) VolumeMultiplier 1.0 0.3 "/Game/ProceduralFramework/Extras/FX/ImpactsAttenuation.ImpactsAttenuation" null))

(fn `Spawn Sound`
  (params (Surface :type "EPhysicalSurface Enum" :default "SurfaceType_Default") (VolumeMultiplier :type "Float (single-precision)") (Location :type "Vector Structure"))
  (if (`self.Debug?`)
    (`KismetSystemLibrary.PrintString` (`|GetEnumeratorNameAsString` (`local.Surface`)))
    (else
      (switch `EPhysicalSurface` (`local.Surface`)
        (:`SurfaceType_Default`
          (`self.CasingSound` (`local.VolumeMultiplier`) (`local.Location`) (`self.Concrete`)))))))

(fn `UserConstructionScript`)