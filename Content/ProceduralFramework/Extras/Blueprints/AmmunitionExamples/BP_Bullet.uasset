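; Projectile actor for the ammunition examples that detects impacts by line tracing between its positions on consecutive ticks once FireBullet runs.
; The trace repeats until it hits, and the actor destroys itself after a fixed lifetime.
; A hit spawns sound, particles and a triggered FS_MasterField_Bullet field, then applies damage and reports it via ReportDamageEvent.
; It also pushes physics-simulating components using bullet velocity and notifies any BP_FiringTarget it strikes.
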(event `Fire Bullet`
  (bind _returnvalue (`GameplayStatics.GetPlayerCharacter` 0))
  (bind _damage (`self.Damage`))
  (bind (_bblockinghit _binitialoverlap _time _distance _location _impactpoint _normal _impactnormal _physmat _hitactor _hitcomponent) (`GameplayStatics.BreakHitResult` (`self.Out Hit`)))
  (`|ExecutionSequence`
    (:`then_0`
      ;[0 0 0] Get the initial location of the projectile
      (set `self.Start Trace` (`self.K2_GetActorLocation`) :!label _label)
      ;[0 0 0] GET LOCATION AFTER SINGLE FRAME
      (`KismetSystemLibrary.DelayUntilNextTick`)
      (set `self.End Trace` (`self.K2_GetActorLocation`))
      ;[0 0 0] CREATE LINE TRACE FROM BOTH LOCATIONS
      (bind (_outhit _returnvalue_2) (`KismetSystemLibrary.LineTraceSingle` :`Start` (`self.Start Trace`) :`End` (`self.End Trace`) :`TraceChannel` "TraceTypeQuery1" :`DrawDebugType` (`self.Debug Path`)))
      (set `self.Out Hit` _outhit)
      (bind _output_get (set `self.Hit?` _returnvalue_2))
      (if _output_get
        (`GameplayStatics.PlaySoundAtLocation` "/Game/ProceduralFramework/Extras/Blueprints/AmmunitionExamples/SW_BulletHit.SW_BulletHit" _location (`KismetMathLibrary.MakeRotFromX` _location) 1.0 1.0 0.2 null null null null)
        (`GameplayStatics.SpawnEmitterAtLocation` "/Game/ProceduralFramework/Extras/FX/Particles/P_Impact.P_Impact" _location (`KismetMathLibrary.MakeRotFromX` _normal))
        (bind _returnvalue_3 (`|SpawnActorFromClass` "/Game/FPSTutorial/Core/FS_MasterField_Bullet.FS_MasterField_Bullet_C" (`KismetMathLibrary.MakeTransform` _location (`KismetMathLibrary.MakeRotFromX` _normal)) "AlwaysSpawn" "MultiplyWithRoot" null null))
        (`/Engine/EditorResources/FieldNodes/FS_MasterField.CE_Trigger` _returnvalue_3)
        (`GameplayStatics.ApplyDamage` _hitactor _damage (`GameplayStatics.GetPlayerController` 0))
        (`AISense_Damage.ReportDamageEvent` _hitactor _returnvalue _damage (`self.K2_GetActorLocation` _returnvalue) _location)
        (`self.ApplyImpulseIfPhys`)
        (bind _asbp_firing_target (cast `/Game/ProceduralFramework/Extras/Blueprints/FiringTarget/BP_FiringTarget` _hitactor))
        (`/Game/ProceduralFramework/Extras/Blueprints/FiringTarget/BP_FiringTarget.Target HIt` _asbp_firing_target)
        (else
          (goto _label))))
    (:`then_1`
      (`KismetSystemLibrary.Delay` 4.0)
      (`self.K2_DestroyActor`))))

(event `ApplyImpulseIfPhys`
  (bind (_bblockinghit _binitialoverlap _time _distance _location _impactpoint _normal _impactnormal _physmat _hitactor _hitcomponent) (`GameplayStatics.BreakHitResult` (`self.Out Hit`)))
  (if (`SceneComponent.IsSimulatingPhysics` _hitcomponent "None")
    (`PrimitiveComponent.AddImpulseAtLocation` _hitcomponent (* (`self.GetVelocity`) (5.0 5.0 5.0)) _location "None")))

(fn `UserConstructionScript`)