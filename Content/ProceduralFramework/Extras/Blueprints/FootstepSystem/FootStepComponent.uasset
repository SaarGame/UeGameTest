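; Footstep component for Characters that plays surface-dependent sounds and particles, with FootTrace intended for AnimNotify calls.
; FootTrace finds the left or right foot socket from FootConfig, traces downward and reads the hit's physical surface.
; That surface selects an attached sound, with speed-scaled volume and a footstep-type parameter, and a pooled particle system aligned to the hit normal.
; Particles require sounds enabled; Debug adds trace drawing and messages.
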(event `FootstepFX`
  (bind _character (`self.Character`))
  (bind ((`Feet_13_14DE26974BB5D7A91410459DE8F3FCE4` _feet) (`FootstepSound_5_D7BAA6B543F22148D71572B467C4B7A5` _footstepsound)) (break `/Game/ProceduralFramework/Extras/Blueprints/FootstepSystem/Data/FootstepConfig` (`self.FootConfig`)))
  (bind (_bblockinghit _binitialoverlap _time _distance _location _impactpoint _normal) (`GameplayStatics.BreakHitResult` (`self.Hit`)))
  (bind (_bblockinghit_2 _binitialoverlap_2 _time_2 _distance_2 _location_2 _impactpoint_2 _normal_2) (`GameplayStatics.BreakHitResult` (`self.Hit`)))
  (bind (_value _returnvalue) (`BlueprintMapLibrary.Map_Find` (`.FootstepParticle_8_74EE15424033DD652A0CB197E2938B2B` (break `/Game/ProceduralFramework/Extras/Blueprints/FootstepSystem/Data/FootstepConfig` (`self.FootConfig`))) (`self.Surface Type`)))
  (bind (_value_2 _returnvalue_2) (`BlueprintMapLibrary.Map_Find` _footstepsound (`self.Surface Type`)))
  (if (`self.Debug`)
    (`KismetSystemLibrary.PrintText` (`|FormatText` "Footstep::     Surface:{0}   Foot:{1}" (`|GetEnumeratorNameAsString` (`self.Surface Type`)) (`self.CurrentFoot`)) (`self.Debug`) true (struct :`G` 0.66 :`B` 1.0 :`A` 1.0) 0.5))
  (if (`self.UseFootstepSounds?`)
    (if _returnvalue_2
      (bind _returnvalue_3 (`GameplayStatics.SpawnSoundAttached` _value_2 (select `bool` (`KismetSystemLibrary.IsValid` _character) :`false` (`Actor.RootComponent` (`self.GetOwner`)) :`true` (`Character.Mesh` _character) :!type "SceneComponent Object Reference") (`BlueprintMapLibrary.Map_Find` _feet (`self.CurrentFoot`)) _location_2 (`KismetMathLibrary.MakeRotFromZ` _normal_2) "SnapToTarget" false (* (`self.UpdateVolume`) 1.0) 1.0 0.0 null null))
      (bind _output_get (set `self.FootstepSound` _returnvalue_3))
      (`/Engine/EditorBlueprintResources/StandardMacros.IsValid` _output_get
        (:`Is Valid`
          (`AudioComponent.SetIntParameter` _output_get "FootstepType" (`KismetMathLibrary.Conv_ByteToInt` (`self.FootstepType`)))
          (if (`self.UseFootstepParticle?`)
            (if _returnvalue
              (`NiagaraFunctionLibrary.SpawnSystemAtLocation` _value _location (`KismetMathLibrary.MakeRotFromZ` _normal) (select `byte` (`self.FootstepType`) :`0` (0.0 0.0 0.0) :`1` (0.0 0.0 0.0) :`2` (0.0 0.0 0.0) :`3` (0.0 0.0 0.0) :`4` (0.0 0.0 0.0) :!type "Vector Structure") true true "AutoRelease"))))
        (:`Is Not Valid`
          (`KismetSystemLibrary.PrintString` "NO AUDIO FOUND" true false (struct :`R` 0.635417 :`A` 1.0)))))))

(event `self.ReceiveBeginPlay`
  ;[0 0 0] Begin Play
  (`KismetSystemLibrary.DelayUntilNextTick`)
  (bind _ascharacter (cast `Character` (`self.GetOwner`)))
  (bind _output_get (set `self.Character` _ascharacter))
  (set `self.Mesh` (`Character.Mesh` _output_get)))

(fn `FindSocketFromName`
  (params (StoredFootName :type Name) (Mesh :type "SceneComponent Object Reference"))
  (returns (`Found?` :type Boolean) (SocketName :type Name))
  (bind (_value _returnvalue) (`BlueprintMapLibrary.Map_Find` (`.Feet_13_14DE26974BB5D7A91410459DE8F3FCE4` (break `/Game/ProceduralFramework/Extras/Blueprints/FootstepSystem/Data/FootstepConfig` (`self.FootConfig`))) StoredFootName))
  (return (and (`SceneComponent.DoesSocketExist` Mesh _value) _returnvalue) _value))

(fn `Foot Trace`
  (params (TraceLength :type "Float (double-precision)") (FootstepType :type "/Game/ProceduralFramework/Component/PFFComp/Enums/E_FootstepType Enum" :default "NewEnumerator0") (FootstepPlacement :type "/Game/ProceduralFramework/Component/PFFComp/Enums/E_FootstepPlacement Enum" :default "NewEnumerator0"))
  (bind _debug (`self.Debug`))
  (bind _mesh (`self.Mesh`))
  (bind _debug_2 (`self.Debug`))
  (bind (_found_ _socketname) (`self.FindSocketFromName` (`self.CurrentFoot`) _mesh))
  (bind _returnvalue (`SceneComponent.GetSocketLocation` _mesh _socketname))
  (set `self.FootstepType` FootstepType)
  (bind _output_get (set `self.FootstepPlacement` FootstepPlacement))
  (switch `/Game/ProceduralFramework/Component/PFFComp/Enums/E_FootstepPlacement` _output_get
    (:`NewEnumerator1`
      (set `self.CurrentFoot` "L"))
    (:`NewEnumerator2`
      (set `self.CurrentFoot` "R")))
  (if _found_
    ;[0 0 0] TRACE
    (bind (_outhit _returnvalue_2) (`KismetSystemLibrary.LineTraceSingle` _returnvalue (+ _returnvalue (`KismetMathLibrary.MakeVector` 0.0 0.0 (* -1 (`local.TraceLength`)))) "TraceTypeQuery1" (`self.FootTraceComplex?`) (`|MakeArray` (`self.GetOwner`)) (select `bool` (`self.Debug`) :`true` "ForDuration" :!type "EDrawDebugTrace Enum") true (struct :`R` 1.0 :`A` 1.0) (struct :`G` 1.0 :`A` 1.0) 1.0))
    (bind _output_get_2 (set `self.Hit` _outhit))
    (if _returnvalue_2
      (bind (_bblockinghit _binitialoverlap _time _distance _location _impactpoint _normal _impactnormal _physmat) (`GameplayStatics.BreakHitResult` _output_get_2))
      (set `self.Surface Type` (`PhysicalMaterial.SurfaceType` _physmat))
      ;[0 0 0] Draw Debug
      (if (`self.Debug`)
        (`KismetSystemLibrary.DrawDebugSphere` _impactpoint 16.0 6 (struct :`R` 1.0 :`G` 1.0 :`B` 1.0 :`A` 1.0) 0.5 1.0))
      (`self.FootstepFX`)
      (return)
      (else
        (`KismetSystemLibrary.PrintString` "Nothing under the feet" _debug _debug (struct :`G` 0.66 :`B` 1.0 :`A` 1.0) 0.0)
        (return)))
    (else
      (`KismetSystemLibrary.PrintString` "Foot Bone Not Found [Place in Animation]" _debug_2 _debug_2 (struct :`R` 0.614583 :`B` 0.003242 :`A` 1.0) 0.3))))

(fn `UpdateVolume`
  (returns (OutVolume :type "Float (double-precision)"))
  (return (`KismetMathLibrary.MapRangeClamped` (`KismetMathLibrary.VSize` (`Actor.GetVelocity` (`self.GetOwner`))) (`self.MinSpeed`) (`self.MaxSpeed`) 0.1 1.0)))